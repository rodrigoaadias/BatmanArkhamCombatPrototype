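; Player controller that switches the view to a cinematic camera for the game's final sequence.
; On BeginPlay it binds to the SGameMode final sequence start and end events and spawns a BP_FinalSequenceCameraActor.
; When the sequence starts, it aims that camera using the controlled pawn and target enemy, then makes it the view target.
; When the sequence ends, it waits briefly before returning the view to the pawn.
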(event `self.ReceiveBeginPlay`
  (bind _assgame_mode (cast `SGameMode` (`GameplayStatics.GetGameMode`)))
  (add `SGameMode.OnFinalSequenceStarted` _assgame_mode (delegate `HandleFinalSequenceStarted`))
  (add `SGameMode.OnFinalSequenceEnded` _assgame_mode (delegate `HandleFinalSequenceEnded`))
  (bind _returnvalue (`|SpawnActorFromClass` "/Game/BP_FinalSequenceCameraActor.BP_FinalSequenceCameraActor_C" (`KismetMathLibrary.MakeTransform` (0.0 0.0 0.0)) "AlwaysSpawn" "MultiplyWithRoot" null null))
  (set `self.CineCamera` _returnvalue))

(event `HandleFinalSequenceEnded`
  (params (TargetEnemy :type "Actor Object Reference"))
  (`KismetSystemLibrary.Delay` 1.0)
  (`self.SetViewTargetWithBlend` (`self.K2_GetPawn`)))

(event `HandleFinalSequenceStarted`
  (params (TargetEnemy :type "Actor Object Reference"))
  (`/Game/BP_FinalSequenceCameraActor.Set Look At Actor` (`self.CineCamera`) (`self.K2_GetPawn`) TargetEnemy)
  (`self.SetViewTargetWithBlend` (`self.CineCamera`)))

(fn `UserConstructionScript`)