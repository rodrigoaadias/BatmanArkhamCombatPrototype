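; Cine camera actor for the final sequence, framing the player and an enemy from the side.
; SetLookAtActor places it slightly toward the player from the enemy, offset perpendicular to their line by CameraDistance, then sets look-at tracking to the player.
; Placement happens once per call, as the per-tick follow logic is disconnected.
; The game mode's final-sequence-ended event clears the now-unused UpdatePosition flag.
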(event `self.ReceiveBeginPlay`
  (bind _assgame_mode (cast `SGameMode` (`GameplayStatics.GetGameMode`)))
  (add `SGameMode.OnFinalSequenceEnded` _assgame_mode (delegate `FinishSequence`)))

(event `FinishSequence`
  (params (TargetEnemy :type "Actor Object Reference"))
  (set `self.UpdatePosition` false))

(event `self.ReceiveTick`
  (params (DeltaSeconds :type "Float (single-precision)")))

(fn `Set Look At Actor`
  (params (Player :type "Actor Object Reference") (Enemy :type "Actor Object Reference"))
  (locals (LocalLookAtSettings :type "CameraLookatTrackingSettings Structure"))
  (bind (_lookattrackingsettings_benablelookattracking _lookattrackingsettings_bdrawdebuglookattrackingposition _lookattrackingsettings_lookattrackinginterpspeed _lookattrackingsettings_actortotrack _lookattrackingsettings_relativeoffset _lookattrackingsettings_ballowroll) (break `CameraLookatTrackingSettings` (`self.LookatTrackingSettings`)))
  (`self.SetCameraPosition` Player Enemy)
  (set `self.LookatTrackingSettings` (make `CameraLookatTrackingSettings` _lookattrackingsettings_benablelookattracking _lookattrackingsettings_bdrawdebuglookattrackingposition _lookattrackingsettings_lookattrackinginterpspeed (`|ConvertAsset` Player) _lookattrackingsettings_relativeoffset _lookattrackingsettings_ballowroll)))

(fn `SetCameraPosition`
  (params (Player :type "Actor Object Reference") (Enemy :type "Actor Object Reference"))
  (bind _returnvalue (`self.K2_GetActorLocation` Enemy))
  (bind _returnvalue_2 (`KismetMathLibrary.Normal` (- _returnvalue (`self.K2_GetActorLocation` Player))))
  (`self.K2_SetActorLocation` (+ (- _returnvalue (* _returnvalue_2 30.0)) (* (`KismetMathLibrary.RotateAngleAxis` _returnvalue_2 90.0 (0.0 0.0 1.0)) (`self.CameraDistance`))) false true))

(fn `UserConstructionScript`)